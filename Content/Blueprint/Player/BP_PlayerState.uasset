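; Player state Blueprint that tracks a player's kills, deaths and kill/death ratio.
; ROS_UpdateKills and UpdateDeaths increment their counters, call CalculateKD, then print the new total with the player name.
; CalculateKD divides kills by deaths, falling back to the kill count while deaths are zero.
; BeginPlay resets only the death counter.
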(event Custom|CalculateKD
  (if (> (Variables|Default|GetDeath) 0)
    (Variables|Default|SetKD (/ (Math|Conversions|ToFloat(Integer) (Variables|Default|GetKills)) (Variables|Default|GetDeath)))
    (else
      (Variables|Default|SetKD (Math|Conversions|ToFloat(Integer) (Variables|Default|GetKills))))))

(event Custom|ROS_UpdateKills
  (bind _result (Math|Integer|IncrementInt (Variables|Default|GetKills))
    (:%20%20
      (bind _output_get (Variables|Default|SetKills _result))
      (CallFunction|CalculateKD)
      (Development|PrintString (Utilities|String|Append "Kills: " (Utilities|String|ToString(Integer) _output_get) (PlayerState|GetPlayerName))))))

(event Custom|UpdateDeaths
  (bind _result (Math|Integer|IncrementInt (Variables|Default|GetDeath))
    (:%20%20
      (bind _output_get (Variables|Default|SetDeath _result))
      (CallFunction|CalculateKD)
      (Development|PrintString (Utilities|String|Append "Deaths: " (Utilities|String|ToString(Integer) _output_get) (PlayerState|GetPlayerName))))))

(event EventBeginPlay
  (Variables|Default|SetDeath 0))

(event EventTick
  (params (DeltaSeconds :type Float%20%28single-precision%29)))

(fn ConstructionScript)