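; Shooter game mode Blueprint that respawns players as military characters at spawn points.
; BeginPlay caches every BP_SpawnPoint actor in the level.
; RespawnPlayer picks one at random, spawns a BP_CharacterMilitary at its location and rotation, and has the given controller possess it, or prints a reminder if none exist.
; The spawn point's availability flag is left unused, so occupied points are not filtered out.
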(event EventBeginPlay
  (bind _outactors (Actor|GetAllActorsOfClass "/Game/Blueprint/BP_SpawnPoint.BP_SpawnPoint_C"))
  (Variables|Default|SetSpawnPoints _outactors))

(event EventTick
  (params (DeltaSeconds :type Float%20%28single-precision%29)))

(fn ConstructionScript)

(fn RespawnPlayer
  (params (PlayerController :type Player%20Controller%20Object%20Reference))
  (if (> (Utilities|Array|Length (Variables|Default|GetSpawnPoints)) 0)
    (bind _output_get (LocalVariables|SetSpawnPoint (.OutItem (Utilities|Array|Random (Variables|Default|GetSpawnPoints)))))
    (bind _returnvalue (Game|SpawnActorfromClass "/Game/Blueprint/Character/BP_CharacterMilitary.BP_CharacterMilitary_C" (Math|Transform|MakeTransform (Transformation|GetActorLocation (LocalVariables|GetSpawnPoint)) (Transformation|GetActorRotation (LocalVariables|GetSpawnPoint)) "1.000000,1.000000,1.000000") "Undefined" "MultiplyWithRoot" 0 0))
    (bind _output_get_2 (LocalVariables|SetNewSpawnedCharacter _returnvalue))
    (Pawn|Possess PlayerController _output_get_2)
    (else
      (Development|PrintString "Add BP_SpawnPoint"))))